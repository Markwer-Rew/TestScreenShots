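; BP_Car is a car pawn that wanders the level on its own using the navigation mesh.
; On BeginPlay it caches the RecastNavMesh and starts Move, which waits briefly, then runs AIMoveTo toward a random reachable point within a radius of its current location.
; Each successful move calls Move again to form an endless roaming loop, while a failed move prints a debug string and ends it.
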(event Custom|Move
  (Utilities|FlowControl|Delay 0.2)
  (AI|AIMoveTo self (.RandomLocation (AI|Navigation|GetRandomReachablePointinRadius (Transformation|GetActorLocation self) 5e+03 (Variables|Default|GetNav) 0)) 0 5.0 false
    (:OnSuccess
      (CallFunction|Move))
    (:OnFail
      (Development|PrintString "Hello"))))

(event EventBeginPlay
  (Utilities|FlowControl|Sequence
    (:then_0
      (bind _returnvalue (Actor|GetActorOfClass "/Script/NavigationSystem.RecastNavMesh"))
      (Variables|Default|SetNav _returnvalue))
    (:then_1
      (CallFunction|Move))))

(fn ConstructionScript)