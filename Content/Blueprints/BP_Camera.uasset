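; BP_Camera is a camera pawn that the first player controller possesses when play begins.
; On BeginPlay it sets that controller's view target to its Target actor, then possesses itself.
; It then attaches itself to Target, if valid, keeping its world transform.
; Tick only checks that Target is valid and takes no action.
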(event EventTick
  (params (DeltaSeconds :type Float%20%28single-precision%29))
  (Variables|Default|GetTarget
    (:then)
    (:else)))

(event EventBeginPlay
  (bind _returnvalue (Game|GetPlayerController 0))
  (Utilities|FlowControl|Sequence
    (:then_0
      (Game|Player|SetViewTargetwithBlend _returnvalue (Variables|Default|GetTarget) 0.0 "VTBlend_Linear" 0.0 false)
      (Pawn|Possess _returnvalue self))
    (:then_1
      (Variables|Default|GetTarget
        (:then
          (Transformation|AttachActorToActor (Variables|Default|GetTarget) "None" "KeepWorld" "KeepWorld" "KeepWorld" true))
        (:else)))))

(fn ConstructionScript)